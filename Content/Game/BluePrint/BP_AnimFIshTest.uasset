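; BP_AnimFIshTest is an actor that moves along a referenced spline once play begins, apparently a test for fish animation.
; The MoveFishT timeline, with play rate set from TimeToCompleteSeconds, lerps distance over the spline's length to set the actor's transform.
; Location is sampled in world space but rotation in local space.
; The GetActorOfClass lookup assigning SplineREF is disconnected, so this graph never sets that reference.
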(event `self.ReceiveBeginPlay`
  (`self.MoveFish`))

(event `MoveFish`
  (bind _spline (`/Game/Game/Blueprint/BP_SplineFIsh.Spline` (`self.SplineREF`)))
  (`TimelineComponent.SetPlayRate` (`self.MoveFishT`) (/ 1.0 (`self.TimeToCompleteSeconds`)))
  (bind (_direction _movetrack) (`Timeline|MoveFishT`)
    (:`Update`
      (bind _returnvalue (`KismetMathLibrary.Lerp` 0.0 (`SplineComponent.GetSplineLength` _spline) _movetrack))
      (`self.K2_SetActorTransform` (`KismetMathLibrary.MakeTransform` (`SplineComponent.GetLocationAtDistanceAlongSpline` _spline _returnvalue "World") (`SplineComponent.GetRotationAtDistanceAlongSpline` _spline _returnvalue "Local"))))))

(fn `UserConstructionScript`)