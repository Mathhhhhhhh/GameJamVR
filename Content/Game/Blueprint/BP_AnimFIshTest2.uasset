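; Test actor that animates a fish along a spline path.
; On BeginPlay it gathers all BP_SplineFIsh actors, then plays a timeline whose rate is set by a completion time in seconds.
; Each update maps the timeline alpha to distance along the first spline only, setting world-space location and local-space rotation.
; A single-actor lookup is left unconnected.
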(event `self.ReceiveBeginPlay`
  (bind _outactors (`GameplayStatics.GetAllActorsOfClass` "/Game/Game/Blueprint/BP_SplineFIsh.BP_SplineFIsh_C"))
  (bind _output_get (set `self.SplineREFArray` _outactors))
  (`self.MoveFish` _output_get))

(event `MoveFish`
  (params (AllMoveFIsh :type "Array of Actor Object Reference"))
  (bind _spline (`/Game/Game/Blueprint/BP_SplineFIsh.Spline` (`|GetArrayItem` (`self.SplineREFArray`))))
  (`TimelineComponent.SetPlayRate` (`self.MoveFishT`) (/ 1.0 (`self.TimeToCompleteSeconds`)))
  (bind (_direction _movetrack) (`Timeline|MoveFishT`)
    (:`Update`
      (bind _returnvalue (`KismetMathLibrary.Lerp` 0.0 (`SplineComponent.GetSplineLength` (`/Game/Game/Blueprint/BP_SplineFIsh.Spline` (`|GetArrayItem` (`self.SplineREFArray`)))) _movetrack))
      (`self.K2_SetActorTransform` (`KismetMathLibrary.MakeTransform` (`SplineComponent.GetLocationAtDistanceAlongSpline` _spline _returnvalue "World") (`SplineComponent.GetRotationAtDistanceAlongSpline` _spline _returnvalue "Local"))))))

(fn `UserConstructionScript`)