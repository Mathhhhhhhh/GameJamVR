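; BP_Guppy is a guppy species actor that turns its mesh to face the direction it moves.
; Each tick, it reads the InterpToMovement velocity and builds a target rotation with world Z as the primary axis, keeping the fish level.
; The mesh's world rotation eases linearly toward that target with a delta-time-scaled alpha, smoothing turns.
; BeginPlay and construction only call the parent class.
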(event `self.ReceiveBeginPlay`
  (`parent.ReceiveBeginPlay`))

(event `self.ReceiveTick`
  (params (DeltaSeconds :type "Float (single-precision)"))
  (bind _mesh (`self.Mesh`))
  (`SceneComponent.K2_SetWorldRotation` _mesh (`|EaseFunction` "Linear" (* DeltaSeconds 2.0) (`SceneComponent.K2_GetComponentRotation` _mesh) (`KismetMathLibrary.MakeRotFromZX` (0.0 0.0 1.0) (`MovementComponent.Velocity` (`self.InterpToMovement`)))) false false))

(fn `UserConstructionScript`
  (`parent.UserConstructionScript`))